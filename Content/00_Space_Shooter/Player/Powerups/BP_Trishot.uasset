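; Trishot powerup pickup for the space shooter player.
; On overlap with a BP_SS_Character, it stores that character as Player and calls TrishotPower with it, then destroys itself after a short delay.
; Overlaps from other actors are ignored, and BeginPlay, Tick and construction only call the parent versions.
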(event `self.ReceiveBeginPlay`
  (`parent.ReceiveBeginPlay`))

(event `self.ReceiveActorBeginOverlap`
  (params (OtherActor :type "Actor Object Reference"))
  (bind _asbp_ss_character (cast `/Game/00_Space_Shooter/Player/BP_SS_Character` OtherActor))
  (bind _output_get (set `self.Player` _asbp_ss_character))
  (`self.TrishotPower` _output_get)
  (`KismetSystemLibrary.Delay` 0.2)
  (`self.K2_DestroyActor`))

(event `self.ReceiveTick`
  (params (DeltaSeconds :type "Float (single-precision)"))
  (`parent.ReceiveTick` DeltaSeconds))

(fn `UserConstructionScript`
  (`parent.UserConstructionScript`))