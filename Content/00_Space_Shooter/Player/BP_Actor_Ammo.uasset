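; BP_Actor_Ammo is a projectile for the space shooter that explodes when it overlaps other actors.
; Tick moves it along its forward vector by Speed scaled with delta time, without sweeping.
; Overlaps with Pawns or actors tagged Pickup are ignored.
; Any other overlap spawns an explosion emitter, plays a 2D sound and destroys the projectile after a brief delay, applying no damage itself.
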(event `self.ReceiveActorBeginOverlap`
  (params (OtherActor :type "Actor Object Reference"))
  ;[1 1 1] On Collision
  (if (not (`self.ActorHasTag` OtherActor "Pickup"))
    (cast `Pawn` OtherActor
      (:`CastFailed`
        (`GameplayStatics.SpawnEmitterAtLocation` "/Game/Realistic_Starter_VFX_Pack_Vol2/Particles/Explosion/P_Explosion_Big_C.P_Explosion_Big_C" (`self.K2_GetActorLocation`))
        (`GameplayStatics.PlaySound2D` "/Game/00_Space_Shooter/Sounds/super-explosion.super-explosion" 1.0 1.0 0.0 null null)
        (`KismetSystemLibrary.Delay` 0.02)
        (`self.K2_DestroyActor`)))))

(event `self.ReceiveTick`
  (params (DeltaSeconds :type "Float (single-precision)"))
  ;[1 1 1] Update Movement
  (`self.K2_SetActorLocation` (+ (`self.K2_GetActorLocation`) (* (`self.GetActorForwardVector`) (* DeltaSeconds (`self.speed`))))))

(fn `UserConstructionScript`)