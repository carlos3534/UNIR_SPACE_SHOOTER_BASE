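; Player character for the space shooter, handling movement, firing, lives and quitting on Escape.
; Enhanced Input drives planar movement and a fire action that spawns BP_Actor_Ammo at FireSpawn, with a timer-reset flag enforcing the fire delay.
; Overlapping an "enemy"-tagged actor costs a life through a DoOnce that resets after a delay, giving temporary invulnerability.
; When lives reach zero, it calls GameOver on BP_SS_HUD.
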(event `self.ReceiveBeginPlay`
  ;[1 1 1] Setup Enhanched Input
  (bind _asplayer_controller (cast `PlayerController` (`self.GetController`)))
  (bind _returnvalue (pcsubsystem `EnhancedInputLocalPlayerSubsystem` _asplayer_controller))
  (`/Engine/EditorBlueprintResources/StandardMacros.IsValid` _returnvalue
    (:`Is Valid`
      (`EnhancedInputSubsystemInterface.AddMappingContext` _returnvalue "/Game/00_Space_Shooter/Input/IMC_Player.IMC_Player" 0 (struct)))))

(event `EnhancedInput|/Game/00_Space_Shooter/Input/IA_Player_Fire`
  (params (ActionValue :type Boolean) (ElapsedSeconds :type "Float (double-precision)") (TriggeredSeconds :type "Float (double-precision)") (InputAction :type "InputAction Object Reference" :default "/Game/00_Space_Shooter/Input/IA_Player_Fire.IA_Player_Fire"))
  ;[1 1 1] Execute Fire
  (:`Triggered`
    (if (`self.CanFire`)
      (`self.doFire`)
      (set `self.CanFire` false)
      (`KismetSystemLibrary.K2_SetTimerDelegate` (delegate `EnableFire`) (`self.FireDelay`)))))

(event `EnableFire`
  ;[1 1 1] Execute Fire
  (set `self.CanFire` true))

(event `EnhancedInput|/Game/00_Space_Shooter/Input/IA_Player_Movement`
  (params (ActionValue :type "Vector2D Structure") (ElapsedSeconds :type "Float (double-precision)") (TriggeredSeconds :type "Float (double-precision)") (InputAction :type "InputAction Object Reference" :default "/Game/00_Space_Shooter/Input/IA_Player_Movement.IA_Player_Movement"))
  ;[1 1 1] Execute movement
  (:`Triggered`
    (`self.AddMovementInput` (`self.GetActorRightVector`) ActionValue_X)
    (`self.AddMovementInput` (`self.GetActorForwardVector`) ActionValue_Y)))

(event `PlayerDamage`
  (bind _output_get (set `self.NumLifes` (- (`self.NumLifes`) 1)))
  (if (== _output_get 0)
    (bind _asbp_ss_hud (cast `/Game/00_Space_Shooter/UI/BP_SS_HUD` (`PlayerController.GetHUD` (`GameplayStatics.GetPlayerController` 0))))
    (`/Game/00_Space_Shooter/UI/BP_SS_HUD.GameOver` _asbp_ss_hud)
    (elif (< _output_get 0)
      (set `self.NumLifes` 0))))

(event `self.ReceiveActorBeginOverlap`
  (params (OtherActor :type "Actor Object Reference"))
  ;[1 1 1] Decrement 1 life on Enemy or buller Collision
  (if (`KismetArrayLibrary.Array_Contains` (`Actor.Tags` OtherActor) "enemy")
    (`/Engine/EditorBlueprintResources/StandardMacros.DoOnce` false :!label _label
      (:`Completed`
        (`self.PlayerDamage`)
        (`KismetSystemLibrary.Delay` (`self.InvulnerabilityTime`))
        (goto _label :!via `Reset`)))))

(event `Key|Escape`
  (params (Key :type "Key Structure"))
  (:`Pressed`
    (`KismetSystemLibrary.QuitGame` null "Quit")))

(fn `doFire`
  (`|SpawnActorFromClass` "/Game/00_Space_Shooter/Player/BP_Actor_Ammo.BP_Actor_Ammo_C" (`SceneComponent.K2_GetComponentToWorld` (`self.FireSpawn`)) "Undefined" "MultiplyWithRoot" null null))

(fn `UserConstructionScript`)