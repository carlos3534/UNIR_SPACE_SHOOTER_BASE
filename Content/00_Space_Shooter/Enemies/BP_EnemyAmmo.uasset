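; BP_EnemyAmmo is an enemy projectile in the space shooter that flies along its forward vector at a set speed.
; Tick moves it without sweep.
; Overlapping a Player-tagged actor fires the OnAmmoDestroy dispatcher, then calls EnemyDestroyed on SS_GameMode.
; A delayed self-destroy event exists, but its dispatcher binding is never run in this graph.
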(event `self.ReceiveTick`
  (params (DeltaSeconds :type "Float (single-precision)"))
  ;[1 1 1] Update Movement
  (`self.K2_SetActorLocation` (+ (`self.K2_GetActorLocation`) (* (`self.GetActorForwardVector`) (* DeltaSeconds (`self.Spped`))))))

(event `self.ReceiveActorBeginOverlap`
  (params (OtherActor :type "Actor Object Reference"))
  ;[1 1 1] On Collision
  (if (`KismetArrayLibrary.Array_Contains` (`Actor.Tags` OtherActor) "Player")
    (`self.OnAmmoDestroy`)
    (bind _asss_game_mode (cast `/Game/00_Space_Shooter/SS_GameMode` (`GameplayStatics.GetGameMode`)))
    (`/Game/00_Space_Shooter/SS_GameMode.Enemy Destroyed` _asss_game_mode)))

(event `Destroyed_Event`
  ;[1 1 1] Destroy event
  (`KismetSystemLibrary.Delay` 0.2)
  (`self.K2_DestroyActor`))

(fn `UserConstructionScript`)