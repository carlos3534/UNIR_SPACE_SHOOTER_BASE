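; BP_EnemyS is a space shooter enemy variant that weaves side to side as it advances, tracing an S-shaped path.
; Each Tick sets MovementVector to the actor's forward vector plus its right vector scaled by the sine of game time, then calls the parent Tick.
; BeginPlay, overlap handling and construction only call the parent class.
; The sway phase follows global game time rather than each enemy's spawn time.
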(event `self.ReceiveBeginPlay`
  (`parent.ReceiveBeginPlay`))

(event `self.ReceiveTick`
  (params (DeltaSeconds :type "Float (single-precision)"))
  (set `self.MovementVector` (+ (`self.GetActorForwardVector`) (* (`self.GetActorRightVector`) (`KismetMathLibrary.Sin` (`KismetSystemLibrary.GetGameTimeInSeconds`)))))
  (`parent.ReceiveTick` DeltaSeconds))

(event `self.ReceiveActorBeginOverlap`
  (params (OtherActor :type "Actor Object Reference"))
  (`parent.ReceiveActorBeginOverlap` OtherActor))

(fn `UserConstructionScript`
  (`parent.UserConstructionScript`))