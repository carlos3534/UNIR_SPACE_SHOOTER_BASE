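; Enemy projectile for the space shooter that damages the player on contact.
; Each tick it moves along its forward vector at a speed set by a variable, without sweeping.
; When its capsule overlaps BP_SS_Character, it calls PlayerDamage, spawns a Niagara explosion at its position, plays an explosion sound at the world origin and destroys itself.
; Overlaps with other actors are ignored.
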(event `self.ReceiveTick`
  (params (DeltaSeconds :type "Float (single-precision)"))
  ;[1 1 1] Update Movement
  (`self.K2_SetActorLocation` (+ (`self.K2_GetActorLocation`) (* (`self.GetActorForwardVector`) (* DeltaSeconds (`self.Spped`))))))

(event `self.Capsule.OnComponentBeginOverlap`
  (params (OverlappedComponent :type "PrimitiveComponent Object Reference") (OtherActor :type "Actor Object Reference") (OtherComp :type "PrimitiveComponent Object Reference") (OtherBodyIndex :type Integer) (bFromSweep :type Boolean) (SweepResult :type "HitResult Structure (by ref)"))
  (bind _asbp_ss_character (cast `/Game/00_Space_Shooter/Player/BP_SS_Character` OtherActor))
  (`/Game/00_Space_Shooter/Player/BP_SS_Character.PlayerDamage` _asbp_ss_character)
  (`GameplayStatics.PlaySoundAtLocation` "/Game/StarterContent/Audio/Explosion02.Explosion02" (0.0 0.0 0.0) (struct) 1.0 1.0 0.0 null null null null)
  (`NiagaraFunctionLibrary.SpawnSystemAtLocation` "/Game/00_Space_Shooter/FX/NS_EXPLOSION.NS_EXPLOSION" (`self.K2_GetActorLocation`))
  (`self.K2_DestroyActor`))

(fn `UserConstructionScript`)