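; Enemy rocket for the space shooter that flies at the position the player occupied at spawn, marked by a target indicator.
; BeginPlay starts a smoke sound and eases the sphere to that point with MoveComponentTo, using a fixed travel time above game level 3.
; Overlapping the player or player ammo fires its destroy dispatcher and notifies SS_GameMode.
; Arrival and destruction share one exit: explosion sound, hide, brief delay, destroy.
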(event `self.ReceiveBeginPlay`
  (bind _sphere (`self.Sphere`))
  (bind _returnvalue (`self.K2_GetActorLocation` (`GameplayStatics.GetPlayerPawn` 0)))
  (`SceneComponent.K2_SetWorldLocation` (`self.TargetIndicator`) _returnvalue false true)
  (add `self.OnEnemyDestroy_0` (delegate `Destroyed_Event`))
  (`GameplayStatics.SpawnSoundAttached` "/Game/StarterContent/Audio/Smoke01.Smoke01" _sphere "None" (0.0 0.0 0.0) (struct) "KeepRelativeOffset" true 0.8 1.0 0.0 null null)
  (`self.SetOvertimeByLevel`)
  (`KismetSystemLibrary.MoveComponentTo` _sphere (`KismetMathLibrary.InverseTransformLocation` (`self.GetTransform`) _returnvalue) (struct) false true (`self.OverTime`))
  (`GameplayStatics.SpawnSound2D` "/Game/StarterContent/Audio/Explosion02.Explosion02" 1.0 1.5 0.0 null :!label _label)
  (`self.SetActorHiddenInGame` true)
  (`KismetSystemLibrary.Delay` 0.2)
  (`self.K2_DestroyActor`))

(event `Destroyed_Event`
  (goto _label))

(event `self.ReceiveTick`
  (params (DeltaSeconds :type "Float (single-precision)")))

(event `self.ReceiveActorBeginOverlap`
  (params (OtherActor :type "Actor Object Reference"))
  (bind _tags (`Actor.Tags` OtherActor))
  ;[1 1 1] On Collision
  (if (or (`KismetArrayLibrary.Array_Contains` _tags "Player_ammo") (`KismetArrayLibrary.Array_Contains` _tags "Player"))
    (`self.OnEnemyDestroy_0`)
    (bind _asss_game_mode (cast `/Game/00_Space_Shooter/SS_GameMode` (`GameplayStatics.GetGameMode`)))
    (`/Game/00_Space_Shooter/SS_GameMode.Enemy Destroyed` _asss_game_mode (`self.K2_GetActorLocation`))))

(fn `SetOvertimeByLevel`
  (bind _asss_game_mode (cast `/Game/00_Space_Shooter/SS_GameMode` (`GameplayStatics.GetGameMode`)))
  (bind _level (`/Game/00_Space_Shooter/SS_GameMode.GetGameLevel` _asss_game_mode))
  (if (> _level 3)
    (set `self.OverTime` 1.0)))

(fn `UserConstructionScript`)