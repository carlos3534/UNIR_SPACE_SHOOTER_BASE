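; BP_RandomGenerator is the space shooter's enemy spawner, spawning a random enemy on a looping SpawnTime timer.
; The random roll scales with the game mode's Level, clamped by MaxNumEnemies, to select among three enemy classes.
; Enemies spawn at random components tagged SpawnPoint.
; A Memoria index is meant to avoid repeated points, but pure random nodes re-roll on each evaluation, so repeats remain possible.
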(event `self.ReceiveBeginPlay`
  (`KismetSystemLibrary.K2_SetTimerDelegate` (delegate `Spawn`) (`self.SpawnTime`) true)
  (bind _asss_game_mode (cast `/Game/00_Space_Shooter/SS_GameMode` (`GameplayStatics.GetGameMode`)))
  (set `self.SS Game Mode` _asss_game_mode))

(event `Spawn`
  (`self.SpawnEnemy`))

(fn `Get Class to Spawn`
  (params (type :type Integer))
  (returns (Class :type "Actor Class Reference"))
  (return (select `int` (`KismetMathLibrary.Clamp` type 0 (- (`self.MaxNumEnemies`) 1)) :`0` "/Game/00_Space_Shooter/Enemies/BP_EnemyBase.BP_EnemyBase_C" :`1` "/Game/00_Space_Shooter/Enemies/BP_EnemyH.BP_EnemyH_C" :`2` "/Game/00_Space_Shooter/Enemies/BP_EnemyS.BP_EnemyS_C" :!type "/Game/00_Space_Shooter/Enemies/BP_EnemyBase Class Reference")))

(fn `SpawnEnemy`
  (returns (NewParam :type "Actor Object Reference"))
  (bind _returnvalue (`self.GetComponentsByTag` "/Script/Engine.SceneComponent" "SpawnPoint"))
  (bind _returnvalue_2 (`KismetArrayLibrary.Array_Length` _returnvalue))
  (bind _returnvalue_3 (`KismetMathLibrary.RandomInteger` _returnvalue_2))
  (bind _returnvalue_4 (select `bool` (== _returnvalue_3 (`self.Memoria`)) :`false` _returnvalue_3 :`true` (mod (`KismetMathLibrary.Conv_Int64ToInt` (+ 0 _returnvalue_3)) _returnvalue_2)))
  (bind _class (`self.Get Class to Spawn` (`KismetMathLibrary.RandomInteger` (`/Game/00_Space_Shooter/SS_GameMode.Level` (`self.SS Game Mode`)))))
  (bind _returnvalue_5 (`|SpawnActorFromClass` _class (`SceneComponent.K2_GetComponentToWorld` (`|GetArrayItem` _returnvalue _returnvalue_4)) "Undefined" "MultiplyWithRoot" null null))
  (bind _asbp_enemy_base (cast `/Game/00_Space_Shooter/Enemies/BP_EnemyBase` _returnvalue_5))
  (set `self.Memoria` _returnvalue_4)
  (return _asbp_enemy_base))

(fn `UserConstructionScript`)