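; BP_Hearth is an extra-life pickup in the space shooter that moves along its forward vector every tick without sweeping.
; On capsule overlap with BP_SS_Character, it adds a life unless the count is three, playing a sound and a Niagara burst.
; At three lives, it instead calls VidasMax on the HUD's game widget.
; Both outcomes destroy the pickup, though the latter requires the BP_SS_HUD cast to succeed.
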(event `self.ReceiveTick`
  (params (DeltaSeconds :type "Float (single-precision)"))
  ;[1 1 1] Update Movement
  (`self.K2_SetActorLocation` (+ (`self.K2_GetActorLocation`) (* (`self.GetActorForwardVector`) (* DeltaSeconds (`self.Spped`))))))

(event `self.Capsule.OnComponentBeginOverlap`
  (params (OverlappedComponent :type "PrimitiveComponent Object Reference") (OtherActor :type "Actor Object Reference") (OtherComp :type "PrimitiveComponent Object Reference") (OtherBodyIndex :type Integer) (bFromSweep :type Boolean) (SweepResult :type "HitResult Structure (by ref)"))
  (bind _asbp_ss_character (cast `/Game/00_Space_Shooter/Player/BP_SS_Character` OtherActor))
  (bind _numlifes (`/Game/00_Space_Shooter/Player/BP_SS_Character.NumLifes` _asbp_ss_character))
  (if (!= _numlifes 3)
    (set `/Game/00_Space_Shooter/Player/BP_SS_Character.NumLifes` (+ _numlifes 1) _asbp_ss_character)
    (`GameplayStatics.PlaySoundAtLocation` "/Game/00_Space_Shooter/Sounds/power-up-sound-effects-all-sounds-audiotrimmer.power-up-sound-effects-all-sounds-audiotrimmer" (0.0 0.0 0.0) (struct) 1.0 1.0 0.0 null null null null)
    (`NiagaraFunctionLibrary.SpawnSystemAtLocation` "/Game/Pack_Simple_Particle_Burst/01_Niagara_Systems/NS_Simple_Burst_Level_3.NS_Simple_Burst_Level_3" (`self.K2_GetActorLocation`))
    (else
      (bind _asbp_ss_hud (cast `/Game/00_Space_Shooter/UI/BP_SS_HUD` (`PlayerController.GetHUD` (`GameplayStatics.GetPlayerController` 0))))
      (`/Game/00_Space_Shooter/UI/BP_SS_GameWidget.VidasMax` (`/Game/00_Space_Shooter/UI/BP_SS_HUD.GameWidget` _asbp_ss_hud))))
  (`self.K2_DestroyActor`))

(fn `UserConstructionScript`)