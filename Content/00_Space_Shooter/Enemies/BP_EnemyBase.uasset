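; Base enemy for the space shooter that flies along its initial forward vector and fires automatically.
; Tick moves it by Speed and spawns Ammo at FirePoint, rotated to match the enemy, each time a shot timer exceeds DelayShoot.
; Overlapping a Player-tagged actor triggers the OnEnemyDestroy dispatcher and notifies SS_GameMode.
; The bound destroy event waits briefly, destroys the enemy and has a small chance to spawn a BP_Hearth pickup.
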(event `self.ReceiveBeginPlay`
  ;[1 1 1] Setup initial direction and Destroy Event
  (set `self.MovementVector` (`self.GetActorForwardVector`))
  (add `self.OnEnemyDestroy` (delegate `Destroyed_Event`)))

(event `Destroyed_Event`
  ;[1 1 1] Setup initial direction and Destroy Event
  (`KismetSystemLibrary.Delay` 0.2)
  (`self.K2_DestroyActor`)
  (if (`KismetMathLibrary.RandomBoolWithWeight` 0.1)
    (`|SpawnActorFromClass` "/Game/00_Space_Shooter/Enemies/BP_Hearth.BP_Hearth_C" (`self.GetTransform`) "Undefined" "MultiplyWithRoot" null null)))

(event `self.ReceiveTick`
  (params (DeltaSeconds :type "Float (single-precision)"))
  ;[1 1 1] Update Movement and Fire
  (`self.Move` DeltaSeconds)
  (bind _output_get (set `self.ShotCurrentTime` (+ DeltaSeconds (`self.ShotCurrentTime`))))
  (if (> _output_get (`self.DelayShoot`))
    (set `self.ShotCurrentTime` 0.0)
    (`self.Fire`)))

(event `self.ReceiveActorBeginOverlap`
  (params (OtherActor :type "Actor Object Reference"))
  ;[1 1 1] On Collision
  (if (`KismetArrayLibrary.Array_Contains` (`Actor.Tags` OtherActor) "Player")
    (`self.OnEnemyDestroy`)
    (bind _asss_game_mode (cast `/Game/00_Space_Shooter/SS_GameMode` (`GameplayStatics.GetGameMode`)))
    (`/Game/00_Space_Shooter/SS_GameMode.Enemy Destroyed` _asss_game_mode)))

(fn `Fire`
  (bind _returnvalue (`|SpawnActorFromClass` (`self.Ammo`) (`SceneComponent.K2_GetComponentToWorld` (`self.FirePoint`)) "Undefined" "MultiplyWithRoot" null null))
  (`self.K2_SetActorRotation` _returnvalue (`self.K2_GetActorRotation`) false))

(fn `Move`
  (params (deltaTime :type "Float (double-precision)"))
  (`self.K2_SetActorLocation` (+ (`self.K2_GetActorLocation`) (* (`self.MovementVector`) (* deltaTime (`self.Speed`))))))

(fn `UserConstructionScript`)