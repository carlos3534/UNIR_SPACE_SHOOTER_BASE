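; Health pickup for the space shooter that gives the player one life, capped at their max.
; Each Tick it moves along the forward vector captured at BeginPlay, scaled by Speed, without sweeping.
; Overlap with a "Player"-tagged actor heals player 0's BP_SS_Character, hides the pickup, plays a sound and destroys it after a short delay.
; A DoOnce guard exists but is unconnected, so repeat overlaps are not blocked.
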(event `self.ReceiveBeginPlay`
  (set `self.MovementVector` (`self.GetActorForwardVector`)))

(event `self.ReceiveActorBeginOverlap`
  (params (OtherActor :type "Actor Object Reference"))
  (if (`KismetArrayLibrary.Array_Contains` (`Actor.Tags` OtherActor) "Player")
    (`self.HealLife` 1)
    (`self.SetActorHiddenInGame` true)
    (`GameplayStatics.SpawnSound2D` "/Engine/VREditor/Sounds/VR_shep_scale_up_04.VR_shep_scale_up_04" 1.0 2.0 1.0 null)
    (`KismetSystemLibrary.Delay` 0.2)
    (`self.K2_DestroyActor`)))

(event `self.ReceiveTick`
  (params (DeltaSeconds :type "Float (single-precision)"))
  ;[1 1 1] update Movement
  (`self.Move` DeltaSeconds))

(fn `HealLife`
  (params (Heal_level :type Integer))
  (bind _asbp_ss_character (cast `/Game/00_Space_Shooter/Player/BP_SS_Character` (`GameplayStatics.GetPlayerCharacter` 0)))
  (set `/Game/00_Space_Shooter/Player/BP_SS_Character.NumLifes` (`KismetMathLibrary.Min` (`/Game/00_Space_Shooter/Player/BP_SS_Character.MaxLife` _asbp_ss_character) (+ (`/Game/00_Space_Shooter/Player/BP_SS_Character.NumLifes` _asbp_ss_character) Heal_level)) _asbp_ss_character))

(fn `Move`
  (params (deltaTime :type "Float (double-precision)"))
  (`self.K2_SetActorLocation` (+ (`self.K2_GetActorLocation`) (* (`self.MovementVector`) (* deltaTime (`self.Speed`))))))

(fn `UserConstructionScript`)